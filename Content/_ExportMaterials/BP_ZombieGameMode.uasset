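; Game mode for a wave-based zombie game that spawns the current wave of BP_ZombieGirl enemies on BeginPlay.
; It sizes each wave from CurrentWave, sets the remaining count, then spawns half the total at each of two spawn locations.
; StartGame calls SpawnZombies, which re-enters the same spawn logic.
; The graph contains no wave advancement, and a leftover StartGame call is unconnected.
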(event Custom|StartGame
  (CallFunction|SpawnZombies))

(event Custom|SpawnZombies
  (bind _output_get (Variables|Default|SetZombieTotal (* (Variables|Default|GetCurrentWave) 4)))
  (bind _output_get_2 (Variables|Default|SetZombiesLeft _output_get))
  (bind _index (Utilities|FlowControl|ForLoopwithBreak 0 _output_get_2 :!label _label)
    (:LoopBody
      (if (== _index (/ (Variables|Default|GetZombieTotal) 2))
        (goto _label Break)
        (else
          (Game|SpawnActorfromClass "/Game/_ExportMaterials/zombiepack/BP_ZombieGirl.BP_ZombieGirl_C" (Variables|Default|GetspawnLocation1) "Undefined" 0 0))))
    (:Completed
      (Utilities|FlowControl|ForLoopwithBreak 1 (/ (Variables|Default|GetZombieTotal) 2)
        (:LoopBody
          (Game|SpawnActorfromClass "/Game/_ExportMaterials/zombiepack/BP_ZombieGirl.BP_ZombieGirl_C" (Variables|Default|GetspawnLocation2) "Undefined" 0 0))))))

(event EventBeginPlay
  (bind _output_get (Variables|Default|SetZombieTotal (* (Variables|Default|GetCurrentWave) 4)))
  (bind _output_get_2 (Variables|Default|SetZombiesLeft _output_get))
  (bind _index (Utilities|FlowControl|ForLoopwithBreak 0 _output_get_2 :!label _label)
    (:LoopBody
      (if (== _index (/ (Variables|Default|GetZombieTotal) 2))
        (goto _label Break)
        (else
          (Game|SpawnActorfromClass "/Game/_ExportMaterials/zombiepack/BP_ZombieGirl.BP_ZombieGirl_C" (Variables|Default|GetspawnLocation1) "Undefined" 0 0))))
    (:Completed
      (Utilities|FlowControl|ForLoopwithBreak 1 (/ (Variables|Default|GetZombieTotal) 2)
        (:LoopBody
          (Game|SpawnActorfromClass "/Game/_ExportMaterials/zombiepack/BP_ZombieGirl.BP_ZombieGirl_C" (Variables|Default|GetspawnLocation2) "Undefined" 0 0))))))

(fn ConstructionScript)