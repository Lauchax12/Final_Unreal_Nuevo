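; BP_ZombieGirl is a zombie character that takes point damage and dies.
; On BeginPlay it loads its health from the "Zombie" row of DT_test.
; Each hit subtracts damage and prints health, but death only triggers on a hit arriving when health is already depleted.
; Death sets IsDeath, stops movement, starts the dying montage and destroys the actor immediately, without waiting for completion.
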(event EventBeginPlay
  (bind _returnvalue (Utilities|GetDataTableRow "/Game/FirstPerson/datatable/DT_test.DT_test" "Zombie")
    (:then
      (Variables|Default|SetHealth (Math|Conversions|ToFloat(Integer) (.maxhealth (Utilities|Struct|BreakTest_DataTableStruc _returnvalue)))))))

(event Game|Damage|EventPointDamage
  (params (Damage :type Float%20%28single-precision%29) (DamageType :type Damage%20Type%20Object%20Reference) (HitLocation :type Vector :default "0, 0, 0") (HitNormal :type Vector :default "0, 0, 0") (HitComponent :type Primitive%20Component%20Object%20Reference) (BoneName :type Name :default "None") (ShotFromDirection :type Vector :default "0, 0, 0") (InstigatedBy :type Controller%20Object%20Reference) (DamageCauser :type Actor%20Object%20Reference) (HitInfo :type Hit%20Result%20Structure%20%28by%20ref%29))
  (if (not (Variables|Default|GetIsDeath))
    (if (<= (Variables|Default|GetHealth) 0.0)
      (Variables|Default|SetIsDeath true)
      (Components|Movement|StopMovementImmediately (Variables|Character|GetCharacterMovement))
      (Animation|Montage|PlayMontage (Variables|Character|GetMesh) "/Game/_ExportMaterials/zombiepack/animations/ZombieDyying.ZombieDyying"
        (:then
          (Actor|DestroyActor)))
      (else
        (bind _output_get (Variables|Default|SetHealth (- (Variables|Default|GetHealth) Damage)))
        (Development|PrintString (Utilities|String|ToString(Float) _output_get))))))

(fn ConstructionScript)